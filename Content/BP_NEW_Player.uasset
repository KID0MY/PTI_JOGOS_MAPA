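; Player character Blueprint that handles movement, single-item pickup and NPC dialogue.
; Room trigger overlaps, matched by display name, set axis signs and a Flipped flag that remap movement input between the capsule's forward and right vectors.
; Tick yaws the PlayerPH component toward the camera, billboard-style.
; Interact picks up an overlapped BP_Item tagged PickUpable with a sound, while C sends TalkMessage to overlapping NPCs through BPI_Dialog.
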(event `InputAxis|MoveForward`
  (params (AxisValue :type "Float (single-precision)"))
  (bind _returnvalue (* (* AxisValue (`self.Movement_Y`) (`GameplayStatics.GetWorldDeltaSeconds`)) (`self.MV_Flip_X`)))
  ;[1 1 1] Movement_Old
  (if (`self.flipped`)
    (`self.AddMovementInput` (`SceneComponent.GetForwardVector` (`self.CapsuleComponent`)) _returnvalue)
    (else
      (`self.AddMovementInput` (`SceneComponent.GetRightVector` (`self.CapsuleComponent`)) _returnvalue))))

(event `InputAxis|MoveRight`
  (params (AxisValue :type "Float (single-precision)"))
  (bind _returnvalue (* (* AxisValue (`self.Movement_X`) (`GameplayStatics.GetWorldDeltaSeconds`)) (`self.MV_Flip_Y`)))
  ;[1 1 1] Movement_Old
  (if (`self.flipped`)
    (`self.AddMovementInput` (`SceneComponent.GetRightVector` (`self.CapsuleComponent`)) _returnvalue)
    (else
      (`self.AddMovementInput` (`SceneComponent.GetForwardVector` (`self.CapsuleComponent`)) _returnvalue))))

(event `self.ReceiveTick`
  (params (DeltaSeconds :type "Float (single-precision)"))
  (bind _player_ph (`self.Player_PH`))
  (bind (_returnvalue_roll _returnvalue_pitch _returnvalue_yaw) (`KismetMathLibrary.BreakRotator` (`KismetMathLibrary.FindLookAtRotation` (`SceneComponent.K2_GetComponentLocation` _player_ph) (`SceneComponent.K2_GetComponentLocation` (`Actor.RootComponent` (`GameplayStatics.GetPlayerCameraManager` 0))))))
  ;[1 1 1] player Rotate
  (`SceneComponent.K2_SetWorldRotation` _player_ph (`KismetMathLibrary.MakeRotator` 0.0 0.0 _returnvalue_yaw) false false))

(event `InputAction|Interact`
  (params (Key :type "Key Structure"))
  (bind _overlappingactors (`PrimitiveComponent.GetOverlappingActors` (`self.CapsuleComponent`) "/Game/OBJETOS/BP_Item.BP_Item_C"))
  ;[1 1 1] player pick up item
  (:`Pressed`
    (if (`self.is_holding`)
      (`KismetSystemLibrary.PrintString` (`KismetSystemLibrary.GetDisplayName` (`self.Held_item`)))
      (else
        (for _array_element _overlappingactors
          (if (`self.ActorHasTag` _array_element "PickUpable")
            (set `self.Held_item` _array_element)
            (`self.K2_DestroyActor` _overlappingactors)
            (`GameplayStatics.PlaySound2D` "/Game/SOUNDS/Resident_Evil_4_Herb_Pick_up_Sound_Effect.Resident_Evil_4_Herb_Pick_up_Sound_Effect" 1.0 1.0 0.0 null null)
            (set `self.is_holding` true)
            (break)))))))

(event `Key|C`
  (params (Key :type "Key Structure"))
  (:`Pressed`
    (for _array_element (`self.GetOverlappingActors` "/Game/BP_NPC.BP_NPC_C")
      (if (`KismetSystemLibrary.DoesImplementInterface` _array_element "/Game/DIALOG/BPI_Dialog.BPI_Dialog_C")
        (message `/Game/DIALOG/BPI_Dialog.Talk` _array_element)))))

(event `self.CapsuleComponent.OnComponentBeginOverlap`
  (params (OverlappedComponent :type "PrimitiveComponent Object Reference") (OtherActor :type "Actor Object Reference") (OtherComp :type "PrimitiveComponent Object Reference") (OtherBodyIndex :type Integer) (bFromSweep :type Boolean) (SweepResult :type "HitResult Structure (by ref)"))
  (bind _returnvalue (`KismetSystemLibrary.GetDisplayName` OtherActor))
  ;[1 1 1] room_check
  (`KismetSystemLibrary.PrintString` _returnvalue)
  (if (`KismetStringLibrary.EqualEqual_StrStr` "Remédio" _returnvalue)
    (`KismetSystemLibrary.PrintString` "MV")
    (elif (or (`KismetStringLibrary.EqualEqual_StrStr` "TriggerBox_Banheiro" _returnvalue) (`KismetStringLibrary.EqualEqual_StrStr` "TriggerBox_quarto" _returnvalue) (`KismetStringLibrary.EqualEqual_StrStr` "TriggerBox_QuartoCasal" _returnvalue) (`KismetStringLibrary.EqualEqual_StrStr` "TriggerBox_QuartoCasal" _returnvalue))
      (`KismetSystemLibrary.PrintString` "Foi")
      (set `self.MV_Flip_X` 1.0)
      (set `self.MV_Flip_Y` -1.0)
      (set `self.flipped` false)
      (`KismetSystemLibrary.PrintString` (`KismetStringLibrary.Conv_DoubleToString` (`self.MV_Flip_X`)))
      (`KismetSystemLibrary.PrintString` (`KismetStringLibrary.Conv_BoolToString` (`self.flipped`)) :!label _label)
      (elif (or (`KismetStringLibrary.EqualEqual_StrStr` "TriggerBox_Corredor" _returnvalue) (`KismetStringLibrary.EqualEqual_StrStr` "TriggerBox_Sala_01" _returnvalue) false)
        (set `self.MV_Flip_X` -1.0)
        (set `self.MV_Flip_Y` 1.0)
        (elif (or (`KismetStringLibrary.EqualEqual_StrStr` "TriggerBox_Sala_02" _returnvalue) false)
          (set `self.MV_Flip_X` 1.0)
          (set `self.MV_Flip_Y` -1.0)
          (else
            (set `self.MV_Flip_X` 1.0)
            (set `self.MV_Flip_Y` -1.0)
            (set `self.flipped` true)
            (goto _label)))))))

(fn `player`
  ;[1 1 1] Movement_Old
  (`self.AddMovementInput` (`SceneComponent.GetRightVector` (`self.CapsuleComponent`)) (* (* 0.0 (`self.Movement_X`) (`GameplayStatics.GetWorldDeltaSeconds`)) (`self.MV_Flip_X`))))

(fn `UserConstructionScript`)