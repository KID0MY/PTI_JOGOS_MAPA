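; Point-and-click player controller that steers the controlled pawn toward the spot the player clicks.
; BeginPlay shows the cursor, and a left click stores the Visibility trace hit location under it, without checking for a hit.
; Each click also spawns a short-lived BP_pointInScreen marker there.
; Tick applies half-scale movement input straight toward the stored location, with no pathfinding or arrival check.
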(event `self.ReceiveTick`
  (params (DeltaSeconds :type "Float (single-precision)"))
  (bind _returnvalue (`self.K2_GetPawn`))
  (`Pawn.AddMovementInput` _returnvalue (`KismetMathLibrary.GetDirectionUnitVector` (`self.K2_GetActorLocation` _returnvalue) (`self.NewLocation`)) 0.5 false))

(event `self.ReceiveBeginPlay`
  (set `self.bShowMouseCursor` true))

(event `Key|LeftMouseButton`
  (params (Key :type "Key Structure"))
  (:`Pressed`
    (bind (_hit _location) (`self.GetLocationUnderCursor`))
    (bind _output_get (set `self.NewLocation` _location))
    (bind _returnvalue (`|SpawnActorFromClass` "/Game/NEW_MOVEMENT/Point_and_Click/BP_pointInScreen.BP_pointInScreen_C" (`KismetMathLibrary.Conv_VectorToTransform` _output_get) "AlwaysSpawn" "MultiplyWithRoot" null null))
    (`KismetSystemLibrary.Delay` 0.2)
    (`self.K2_DestroyActor` _returnvalue)))

(fn `GetLocationUnderCursor`
  (returns (Hit :type Boolean) (Location :type "Vector Structure"))
  (bind (_bblockinghit _binitialoverlap _time _distance _location) (`GameplayStatics.BreakHitResult` (`self.GetHitResultUnderCursorByChannel` "TraceTypeQuery1")))
  (return _bblockinghit _location))

(fn `UserConstructionScript`)