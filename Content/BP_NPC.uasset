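; BP_NPC is an NPC Blueprint that shows its dialogue on screen one entry per Talk event.
; Each Talk increments TalkIndex, creates the WB_Dialogue widget if none is valid, and sets its TalkText to that Dialogue entry.
; Once TalkIndex exceeds the Dialogue length, the widget is removed from the viewport, and the index is never reset here.
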(event `/Game/DIALOG/BPI_Dialog.Talk`
  (`/Engine/EditorBlueprintResources/StandardMacros.IncrementInt` (`self.talk_index`)
    (:`  `
      (if (<= (`self.talk_index`) (`KismetArrayLibrary.Array_Length` (`self.dialogue`)))
        (`self.UI`
          (:`then`
            _)
          (:`else`
            (bind _returnvalue (`|CreateWidget` "/Game/DIALOG/WB_Dialogue.WB_Dialogue_C" (`GameplayStatics.GetPlayerController` 0)))
            (bind _output_get (set `self.UI` _returnvalue))
            (`UserWidget.AddToViewport` _output_get 0)))
        (`TextBlock.SetText` (`/Game/DIALOG/WB_Dialogue.Talk_text` (`self.UI`)) (`KismetTextLibrary.Conv_StringToText` (`|GetArrayItem` (`self.dialogue`) (`self.talk_index`))))
        (else
          (`Widget.RemoveFromParent` (`self.UI`)))))))

(fn `UserConstructionScript`)